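; Player character Blueprint that opens and closes the inventory screen through a ToggleInventory event.
; Opening creates a new InventoryWidget, adds it to the viewport, pauses the game and shows the mouse cursor.
; Closing finds top-level InventoryWidgets by class rather than a stored reference, removes them, unpauses, hides the cursor and returns focus to the game viewport.
; An InventoryOpen flag, cleared on BeginPlay, selects between the two branches.
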(event `self.ReceiveBeginPlay`
  (set `self.InventoryOpen` false))

(event `self.ToggleInventory`
  (if (`self.InventoryOpen`)
    (bind _foundwidgets (`WidgetBlueprintLibrary.GetAllWidgetsOfClass` "/Game/HUD/InventoryWidget.InventoryWidget_C"))
    (for _array_element _foundwidgets
      (`Widget.RemoveFromParent` _array_element)
      (set `self.InventoryOpen` false)
      (`GameplayStatics.SetGamePaused` false)
      (set `PlayerController.bShowMouseCursor` false (`GameplayStatics.GetPlayerController` 0))
      (`WidgetBlueprintLibrary.SetFocusToGameViewport`))
    (else
      (bind _returnvalue (`|CreateWidget` "/Game/HUD/InventoryWidget.InventoryWidget_C"))
      (set `self.InventoryOpen` true)
      (`UserWidget.AddToViewport` _returnvalue 0)
      (`GameplayStatics.SetGamePaused` true)
      (set `PlayerController.bShowMouseCursor` true (`GameplayStatics.GetPlayerController` 0)))))

(fn `UserConstructionScript`)